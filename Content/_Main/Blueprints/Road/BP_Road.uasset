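; Road actor that populates its spline with BP_Car actors.
; After a start delay on BeginPlay, a timer fires SpawnCar, which spawns cars in a single loop until the maximum count is reached, then clears the timer.
; All cars spawn at the spline component's location, adjusted for collisions if possible, and receive the spline as their path to follow.
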(event Custom|SpawnCar
  (while (< (Variables|Default|GetNumOfCars) (Variables|Default|GetMaxNumOfCars))
    (Math|Integer|IncrementInt (Variables|Default|GetNumOfCars)
      (:%20%20
        (Game|SpawnActorfromClass "/Game/_Main/Blueprints/Road/BP_Car.BP_Car_C" (Math|Transform|MakeTransform (Transformation|GetWorldLocation (Variables|Default|GetRoadSpline))) "AdjustIfPossibleButAlwaysSpawn" "MultiplyWithRoot" self (Variables|Default|GetRoadSpline) 0))))
  (Utilities|Time|ClearandInvalidateTimerbyHandle (Variables|Default|GetSpawnTimer)))

(event EventBeginPlay
  (Utilities|FlowControl|Delay (Variables|Default|GetTimeToWaitBeforeStart))
  (bind _returnvalue (Utilities|Time|SetTimerbyEvent (delegate Custom|SpawnCar) 2.0 true))
  (Variables|Default|SetSpawnTimer _returnvalue))

(fn ConstructionScript)