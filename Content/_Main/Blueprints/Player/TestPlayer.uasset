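; TestPlayer is a test player character that walks forward automatically every Tick while CanMove is true.
; On BeginPlay it sets a downward camera pitch and installs IMC_Test as the only Enhanced Input mapping context.
; Holding IA_TestMove halts movement and plays the LookDown timeline to drive camera pitch, then reverses it on release.
; Look and move inputs are disconnected, and sprint writes zero to MaxWalkSpeed on press and release.
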(event Input|EnhancedActionEvents|EnhancedInputActionIA_Look
  (params (ActionValue :type Vector%202D%20Structure) (ElapsedSeconds :type Float%20%28double-precision%29) (TriggeredSeconds :type Float%20%28double-precision%29) (InputAction :type Input%20Action%20Object%20Reference :default "/Game/_Main/Blueprints/Player/Input/Actions/IA_Look.IA_Look")))

(event Input|EnhancedActionEvents|EnhancedInputActionIA_Move
  (params (ActionValue :type Vector%202D%20Structure) (ElapsedSeconds :type Float%20%28double-precision%29) (TriggeredSeconds :type Float%20%28double-precision%29) (InputAction :type Input%20Action%20Object%20Reference :default "/Game/_Main/Blueprints/Player/Input/Actions/IA_Move.IA_Move")))

(event Input|EnhancedActionEvents|EnhancedInputActionIA_Sprint
  (params (ActionValue :type Boolean) (ElapsedSeconds :type Float%20%28double-precision%29) (TriggeredSeconds :type Float%20%28double-precision%29) (InputAction :type Input%20Action%20Object%20Reference :default "/Game/_Main/Blueprints/Player/Input/Actions/IA_Sprint.IA_Sprint"))
  (:Started
    (Variables|/Script/Engine.CharacterMovementComponent|SetMaxWalkSpeed (Variables|Character|GetCharacterMovement) (* 0.0 0.0)))
  (:Canceled
    (Variables|/Script/Engine.CharacterMovementComponent|SetMaxWalkSpeed (Variables|Character|GetCharacterMovement) 0.0 :!label _label))
  (:Completed
    (goto _label)))

(event Input|EnhancedActionEvents|EnhancedInputActionIA_TestMove
  (params (ActionValue :type Boolean) (ElapsedSeconds :type Float%20%28double-precision%29) (TriggeredSeconds :type Float%20%28double-precision%29) (InputAction :type Input%20Action%20Object%20Reference :default "/Game/_Main/Blueprints/Player/Input/Actions/Test/IA_TestMove.IA_TestMove"))
  (:Triggered
    (Variables|Default|SetbCanMove false)
    (bind _lookdown (Timeline|LookDown Play)
      (:Update
        (Transformation|SetWorldRotation (Variables|Default|GetCamera) (Math|Rotator|MakeRotator 0.0 _lookdown 0.0) false false))))
  (:Canceled
    (Variables|Default|SetbCanMove true :!label _label)
    (Timeline|LookDown Reverse))
  (:Completed
    (goto _label)))

(event EventTick
  (params (DeltaSeconds :type Float%20%28single-precision%29))
  (if (Variables|Default|GetbCanMove)
    (Pawn|Input|AddMovementInput (Transformation|GetActorForwardVector) 1.0 false)))

(event EventBeginPlay
  (Transformation|SetWorldRotation (Variables|Default|GetCamera) "-30.000000,0.000000,0.000000" false false)
  (bind _asplayer_controller (Utilities|Casting|CastToPlayerController (Pawn|GetController)))
  (Class|EnhancedInputSubsystemInterface|ClearAllMappings (PlayerController|LocalPlayerSubsystems|GetEnhancedInputLocalPlayerSubsystem _asplayer_controller))
  (Input|AddMappingContext (PlayerController|LocalPlayerSubsystems|GetEnhancedInputLocalPlayerSubsystem _asplayer_controller) "/Game/_Main/Blueprints/Player/Input/IMC_Test.IMC_Test" 0 "(bIgnoreAllPressedKeysUntilRelease=True,bForceImmediately=False,bNotifyUserSettings=False)"))

(fn ConstructionScript)